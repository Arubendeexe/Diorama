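; BP_MouseKey is a demo-template prop that displays an animated mouse icon on a widget component to illustrate mouse input.
; On BeginPlay it reveals the widget, optionally loops a timeline that moves it in local Y/Z, and plays a left or right click animation on UIE_Mouse.
; The construction script instead casts the widget to UIE_KeyboardKey to set key text, so it only applies with that widget class.
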(event `self.ReceiveBeginPlay`
  (`SceneComponent.SetVisibility` (`self.Widget`) (`self.Visible In Game`) false)
  (`|ExecutionSequence`
    (:`then_0`
      (if (`self.MoveMouse`)
        (bind (_direction _newtrack_0) (`Timeline|Timeline` :!via `PlayFromStart` :!label _label)
          (:`Update`
            (`SceneComponent.K2_SetRelativeLocation` (`self.Widget`) (`KismetMathLibrary.MakeVector` 0.0 (* (.x _newtrack_0) 25.0) (* (.y _newtrack_0) 25.0)) false false))
          (:`Finished`
            (`KismetSystemLibrary.DelayUntilNextFrame`)
            (goto _label :!via `PlayFromStart`)))))
    (:`then_1`
      (bind _asuie_mouse (cast `/Game/DemoTemplate/_Core/KeyboardKey/UIE_Mouse` (`WidgetComponent.GetWidget` (`self.Widget`))))
      (if (`self.Left Mouse`)
        (`/Game/DemoTemplate/_Core/KeyboardKey/UIE_Mouse.Play Left Click` _asuie_mouse)
        (elif (`self.Right Mouse`)
          (`/Game/DemoTemplate/_Core/KeyboardKey/UIE_Mouse.Play Right Click` _asuie_mouse))))))

(fn `UserConstructionScript`
  (bind _asuie_keyboard_key (cast `/Game/DemoTemplate/_Core/KeyboardKey/UIE_KeyboardKey` (`WidgetComponent.GetWidget` (`self.Widget`))))
  (bind _output_get (set `/Game/DemoTemplate/_Core/KeyboardKey/UIE_KeyboardKey.Key` (`self.Key`) _asuie_keyboard_key))
  (`TextBlock.SetText` (`/Game/DemoTemplate/_Core/KeyboardKey/UIE_KeyboardKey.Text` _asuie_keyboard_key) _output_get))